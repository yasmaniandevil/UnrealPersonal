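; BP_Collect is an unfinished actor Blueprint with scaffolding for movement that never moves the actor.
; Tick stores the current location and plays a timeline whose update lerps toward Target at a fixed zero alpha, writing the result back into Target.
; SetActorLocation is unreachable, and sine and Speed-scaled delta-time math sit unused.
; BeginPlay and overlap events are empty, so no collection logic exists.
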(event EventBeginPlay)

(event Collision|EventActorBeginOverlap
  (params (OtherActor :type Actor%20Object%20Reference)))

(event EventTick
  (params (DeltaSeconds :type Float%20%28single-precision%29))
  (bind _output_get (Variables|Default|SetInitalLocation (Transformation|GetActorLocation)))
  (Timeline|Timeline Play
    (:Update
      (Variables|Default|SetTarget (Math|Vector|Lerp(Vector) _output_get (Variables|Default|GetTarget) 0.0)))))

(fn ConstructionScript)